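; EmitterBP is a laser emitter game piece that can cast a bouncing beam, though its Tick is empty and the CastLight call in its event graph is disconnected.
; CastLight clears old beams, then loops line traces, mirroring off basic wall materials and sending ToggleStateMessage to rust-metal hits.
; Each segment spawns a MasterLaserBP, red or blue by the emitter's own material.
; NewCastLight is an empty stub.
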(event `self.ReceiveTick`
  (params (DeltaSeconds :type "Float (single-precision)")))

(fn `Cast Light`
  (params (CastOrigin :type "Vector Structure") (CastDirection :type "Vector Structure") (CastDistance :type "Float (double-precision)"))
  (locals (CastDistanceLOCAL :type "Float (double-precision)") (CastDirectionLOCAL :type "Vector Structure") (ContinueLOCAL :type Boolean :default true) (CastOriginLOCAL :type "Vector Structure") (BeamStartLOCAL :type "Vector Structure") (BeamEndLOCAL :type "Vector Structure") (NewBeamStartLOCAL :type "Vector Structure") (NewBeamEndLOCAL :type "Vector Structure"))
  (bind _beams (`self.Beams`))
  (bind _castoriginlocal (`local.CastOriginLOCAL`))
  (bind _returnvalue (+ _castoriginlocal (* (`local.CastDirectionLOCAL`) (`local.CastDistanceLOCAL`))))
  (set `local.CastOriginLOCAL` CastOrigin)
  (set `local.CastDirectionLOCAL` CastDirection)
  (set `local.CastDistanceLOCAL` CastDistance)
  (for _array_element _beams
    (`self.K2_DestroyActor` _array_element))
  (`KismetArrayLibrary.Array_Clear` _beams)
  (while (`local.ContinueLOCAL`)
    (`|ExecutionSequence`
      (:`then_0`
        (bind (_outhit _returnvalue_2) (`KismetSystemLibrary.LineTraceSingle` :`Start` _castoriginlocal :`End` _returnvalue :`TraceChannel` "TraceTypeQuery3" :`bTraceComplex` true :`DrawDebugType` "ForDuration" :`DrawTime` 0.01))
        (set `local.BeamStartLOCAL` (`local.CastOriginLOCAL`))
        (if _returnvalue_2
          (bind (_bblockinghit _binitialoverlap _time _distance _location _impactpoint _normal _impactnormal _physmat _hitactor _hitcomponent _hitbonename _hititem _faceindex) (`GameplayStatics.BreakHitResult` _outhit))
          (set `local.BeamEndLOCAL` _impactpoint)
          (bind (_sectionindex _returnvalue_3) (`PrimitiveComponent.GetMaterialFromCollisionFaceIndex` _hitcomponent _faceindex))
          (if (or (== _returnvalue_3 "/Game/StarterContent/Materials/M_Basic_Wall.M_Basic_Wall") (== _returnvalue_3 "/Game/StarterContent/Materials/M_Basic_Wall_Dark.M_Basic_Wall_Dark"))
            (bind _output_get (set `local.CastOriginLOCAL` _impactpoint))
            (bind _returnvalue_4 (`KismetMathLibrary.MirrorVectorByNormal` (`local.CastDirectionLOCAL`) _impactnormal))
            (bind _output_get_2 (set `local.CastDirectionLOCAL` _returnvalue_4))
            (set `local.ContinueLOCAL` true)
            (`KismetSystemLibrary.PrintString` (`KismetStringLibrary.Concat_StrStr` "mirrored : " (`KismetStringLibrary.Conv_VectorToString` _returnvalue_4) " : " (`KismetStringLibrary.Conv_VectorToString` _output_get) " : " (`KismetStringLibrary.Conv_VectorToString` _output_get_2)) true true (struct :`G` 0.66 :`B` 1.0 :`A` 1.0) 0.1)
            (else
              (if (== _returnvalue_3 "/Game/StarterContent/Materials/M_Metal_Rust.M_Metal_Rust")
                (message `/Game/Interfaces/LaserColisionIF.ToggleState` _hitactor true))
              (set `local.ContinueLOCAL` false :!label _label)))
          (else
            (set `local.BeamEndLOCAL` _returnvalue)
            (goto _label))))
      (:`then_2`
        (bind _returnvalue_5 (`|SpawnActorFromClass` "/Game/Lighting/Lasers/MasterLaserBP.MasterLaserBP_C" (`KismetMathLibrary.MakeTransform` (0.0 0.0 0.0)) "Undefined" "OverrideRootScale" null null))
        (`PrimitiveComponent.SetMaterial` (`/Game/Lighting/Lasers/MasterLaserBP.Laser` _returnvalue_5) 0 (select `bool` (== (`PrimitiveComponent.GetMaterial` (`self.StaticMesh`) 0) "/Game/StarterContent/Materials/M_Basic_Wall_Dark.M_Basic_Wall_Dark") :`false` "/Game/Lighting/Lasers/Assets/BlueLaserMaterial.BlueLaserMaterial" :`true` "/Game/Lighting/Lasers/Assets/RedLaserMaterial.RedLaserMaterial" :!type "Material Object Reference"))
        (`/Game/Lighting/Lasers/MasterLaserBP.Set Ends` _returnvalue_5 (`local.BeamStartLOCAL`) (`local.BeamEndLOCAL`))
        (`KismetArrayLibrary.Array_Add` (`self.Beams`) _returnvalue_5)))))

(fn `NewCastLight`
  (params (CastingPiece :type Integer)))

(fn `UserConstructionScript`
  (`parent.UserConstructionScript`))