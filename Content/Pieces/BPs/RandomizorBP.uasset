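; RandomizorBP is a game piece that switches lights on or off, with no randomization in its logic.
; On BeginPlay it adds its PointLight to an AffectedLights array.
; ToggleState forwards the state via ToggleStateMessage to that array and to every PointLight actor found in the world.
; It also sets visibility on those actors' root components and on its own PointLight to match.
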(event `self.ReceiveBeginPlay`
  (`KismetArrayLibrary.Array_Add` (`self.AffectedLights`) (`self.PointLight`)))

(event `/Game/Interfaces/LaserColisionIF.ToggleState`
  (params (`On/Off` :type Boolean))
  (for _array_element (`self.AffectedLights`)
    (message `/Game/Interfaces/LaserColisionIF.ToggleState` _array_element `On/Off`))
  (bind _outactors (`GameplayStatics.GetAllActorsOfClass` "/Script/Engine.PointLight"))
  (for _array_element_2 _outactors
    (message `/Game/Interfaces/LaserColisionIF.ToggleState` _array_element_2 `On/Off`)
    (`SceneComponent.SetVisibility` (`Actor.RootComponent` _array_element_2) `On/Off` false))
  (`SceneComponent.SetVisibility` (`self.PointLight`) `On/Off` false))

(fn `UserConstructionScript`
  (`parent.UserConstructionScript`))