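; Game instance for a multiplayer game with a lobby and chess map, handling session hosting, joining, menus and map travel.
; LaunchLobby creates a non-LAN session, ignoring EnableLAN, then opens LobbyMap as a listen server.
; It counts playing and ready players, creates and caches main and lobby menu widgets, and tells the main menu whether a save exists.
; Network and travel error handlers route to empty string and display stubs.
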(event `StartMatch`
  (`GameplayStatics.OpenLevel` "ChessMap"))

(event `LaunchLobby`
  (params (NumPlayers :type Integer) (EnableLAN :type Boolean) (ServerName :type Text))
  (set `self.MaxPlayers` NumPlayers)
  (set `self.ServerName` ServerName)
  (`CreateSessionCallbackProxy.CreateSession` (`GameplayStatics.GetPlayerController` 0) (`self.MaxPlayers`)
    (:`OnSuccess`
      (`GameplayStatics.OpenLevel` "LobbyMap" true "listen")
      (`self.AddPlayersPlaying`)
      (`KismetSystemLibrary.PrintString` (`KismetStringLibrary.Conv_IntToString` (`self.PlayersPlaying`))))
    (:`OnFailure`
      (`KismetSystemLibrary.PrintString` "failed ya, momma"))))

(event `JoinGame`
  (params (SessionToJoin :type "BlueprintSessionResult Structure (by ref)"))
  (`JoinSessionCallbackProxy.JoinSession` (`GameplayStatics.GetPlayerController` 0) SessionToJoin
    (:`OnSuccess`
      (`self.AddPlayersPlaying`)
      (`KismetSystemLibrary.PrintString` (`KismetStringLibrary.Conv_IntToString` (`self.PlayersPlaying`))))))

(event `AddPlayersPlaying`
  (set `self.PlayersPlaying` (+ (`self.PlayersPlaying`) 1)))

(event `MinusPlayersPlaying`
  (set `self.PlayersPlaying` (+ (`self.PlayersPlaying`) -1)))

(event `AddPlayersReady`
  (bind _output_get (set `self.PlayersReady` (+ (`self.PlayersReady`) 1)))
  (`KismetSystemLibrary.PrintString` (`KismetStringLibrary.Conv_IntToString` _output_get)))

(event `MinusPlayersReady`
  (set `self.PlayersReady` (+ (`self.PlayersReady`) -1)))

(event `LobbyLaserShow`)

(event `self.HandleNetworkError`
  (params (FailureType :type "ENetworkFailure Enum" :default "NetDriverAlreadyExists") (bIsServer :type Boolean))
  ;[1 1 1] NetworkAndTravelErrorProcessing
  (if bIsServer
    _
    (else
      _))
  (`self.DisplayErrorMessage` (`self.NetError -> String` FailureType)))

(event `self.HandleTravelError`
  (params (FailureType :type "ETravelFailure Enum" :default "NoLevel"))
  ;[1 1 1] NetworkAndTravelErrorProcessing
  (`self.DisplayErrorMessage` (`self.TravelError -> String` FailureType)))

(fn `LookForSessions`)

(fn `NetError -> String`
  (params (FailureType :type "ENetworkFailure Enum" :default "NetDriverAlreadyExists"))
  (returns (ErMessage :type String))
  (return ""))

(fn `OnRep_PlayersReady`)

(fn `SaveGameCheck`
  (bind _returnvalue (`GameplayStatics.DoesSaveGameExist` (`self.PlayerSettingsSave`)))
  (if _returnvalue
    (set `self.DoesSaveFileExist?` true)))

(fn `ShowLobbyMenu`
  (bind _returnvalue (`GameplayStatics.GetPlayerController` 0))
  (`/Engine/EditorBlueprintResources/StandardMacros.IsValid` (`self.wLobbyMenu`)
    (:`Is Valid`
      _)
    (:`Is Not Valid`
      (bind _returnvalue_2 (`|CreateWidget` "/Game/UI/LobbyMenu.LobbyMenu_C" _returnvalue))
      (set `self.wLobbyMenu` _returnvalue_2)))
  (`UserWidget.AddToViewport` (`self.wLobbyMenu`) 0)
  (set `PlayerController.bShowMouseCursor` true _returnvalue))

(fn `ShowMainMenu`
  (bind _returnvalue (`GameplayStatics.GetPlayerController` 0))
  (`/Engine/EditorBlueprintResources/StandardMacros.IsValid` (`self.wMainMenu`)
    (:`Is Valid`
      _)
    (:`Is Not Valid`
      (bind _returnvalue_2 (`|CreateWidget` "/Game/UI/MainMenu.MainMenu_C" _returnvalue))
      (set `self.wMainMenu` _returnvalue_2)))
  (set `/Game/UI/MainMenu.SaveGameDetected?` (`self.DoesSaveFileExist?`) (`self.wMainMenu`))
  (`UserWidget.AddToViewport` (`self.wMainMenu`) 0)
  (set `PlayerController.bShowMouseCursor` true _returnvalue))

(fn `TravelError -> String`
  (params (FailureType :type "ETravelFailure Enum" :default "NoLevel"))
  (returns (ErMessage :type String))
  (return ""))