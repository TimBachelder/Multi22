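; ChessBoard is an unfinished chess board Blueprint that spawns a checkered grid of mesh tiles in its construction script, caching each tile's material.
; GetValidMoves pulses two candidate pawn squares; other piece types have no move logic.
; ResetBoardGrid restores cached materials, and PrintArrays dumps debug info.
; Click is an empty stub, with its selection and piece-moving logic left disconnected.
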(fn `Click`
  (params (position :type "Vector Structure")))

(fn `GetValidMoves`
  (params (Index :type Integer))
  (locals (CurrentIndexLOCAL :type Integer) (PieceLOCAL :type "StaticMesh Object Reference") (MaterialLOCAL :type "MaterialInterface Object Reference") (`IsWhitePlayer?` :type Boolean))
  (set `local.CurrentIndexLOCAL` Index)
  (set `local.PieceLOCAL` (`|GetArrayItem` (`self.PiecesMesh`) Index))
  (`/Engine/EditorBlueprintResources/StandardMacros.IsValid` (`local.PieceLOCAL`)
    (:`Is Valid`
      (if (> (`KismetArrayLibrary.Array_Find` (`self.WhitePlayers`) (`local.CurrentIndexLOCAL`)) 0)
        (set `local.IsWhitePlayer?` true)
        (else
          (set `local.IsWhitePlayer?` false)))
      (if (== (`local.PieceLOCAL`) "/Game/Pieces/Assets/Pawn.Pawn")
        (`KismetSystemLibrary.PrintString` "Hello")
        (if (and (== (/ (`local.CurrentIndexLOCAL`) 8) 1) (`local.IsWhitePlayer?`))
          (`PrimitiveComponent.SetMaterial` (`|GetArrayItem` (`self.Field_mesh`) (+ (`self.last_click`) 8)) 0 "/Game/StarterContent/Materials/M_Tech_Hex_Tile_Pulse.M_Tech_Hex_Tile_Pulse")
          (`PrimitiveComponent.SetMaterial` (`|GetArrayItem` (`self.Field_mesh`) (+ (`self.last_click`) 16)) 0 "/Game/StarterContent/Materials/M_Tech_Hex_Tile_Pulse.M_Tech_Hex_Tile_Pulse")
          (return)
          (else
            (`PrimitiveComponent.SetMaterial` (`|GetArrayItem` (`self.Field_mesh`) (+ (`self.last_click`) -8)) 0 "/Game/StarterContent/Materials/M_Tech_Hex_Tile_Pulse.M_Tech_Hex_Tile_Pulse")
            (`PrimitiveComponent.SetMaterial` (`|GetArrayItem` (`self.Field_mesh`) (+ (`self.last_click`) -16)) 0 "/Game/StarterContent/Materials/M_Tech_Hex_Tile_Pulse.M_Tech_Hex_Tile_Pulse")
            (return)))
        (elif (== (`local.PieceLOCAL`) "/Game/Pieces/Assets/Bishop.Bishop")
          _
          (elif (== (`local.PieceLOCAL`) "/Game/Pieces/Assets/Knight.Knight")
            (if (== (`local.PieceLOCAL`) "/Game/Pieces/Assets/Rook.Rook")
              (if (== (`local.PieceLOCAL`) "/Game/Pieces/Assets/Queen.Queen")
                (if (== (`local.PieceLOCAL`) "/Game/Pieces/Assets/King.King")
                  _)))))))))

(fn `PrintArrays`
  (for _index (range 10 21)
    (`KismetSystemLibrary.PrintString` (`KismetStringLibrary.Concat_StrStr` "FieldMesh  :  " (`KismetSystemLibrary.GetDisplayName` (`|GetArrayItem` (`self.Field_mesh`) _index)) "  : F.Material : " (`KismetSystemLibrary.GetDisplayName` (`|GetArrayItem` (`self.Field_material`) _index)) " : PiecesMesh  :" (`KismetSystemLibrary.GetDisplayName` (`|GetArrayItem` (`self.pieces_mesh_Component`) _index)) "  : INDEX  :  " (`KismetStringLibrary.Conv_IntToString` _index)) true true (struct :`G` 0.66 :`B` 1.0 :`A` 1.0) 22.0))
  (return))

(fn `ResetBoardGrid`
  ;[1 1 1 1 14] DrawsBoard
  (for _index (range 81)
    (`PrimitiveComponent.SetMaterial` (`|GetArrayItem` (`self.Field_mesh`) _index) 0 (`|GetArrayItem` (`self.Field_material`) _index))))

(fn `UserConstructionScript`
  ;[1 1 1 1 14] DrawsBoard
  (for _index (range 81)
    (bind _returnvalue (`AddComponent|NODE_AddStaticMeshComponent-0` :`RelativeTransform` (`KismetMathLibrary.Conv_VectorToTransform` (`/Game/Blueprints/Libraries/MathLibrary.Index -> Position` _index))))
    (`KismetArrayLibrary.Array_Add` (`self.Field_mesh`) _returnvalue)
    (bind _returnvalue_2 (select `bool` (xor (`KismetMathLibrary.Conv_IntToBool` (mod _index 2)) (`KismetMathLibrary.Conv_IntToBool` (mod (/ _index 9) 1))) :`false` "/Game/StarterContent/Materials/M_Basic_Wall.M_Basic_Wall" :`true` "/Game/StarterContent/Materials/M_Basic_Wall_Dark.M_Basic_Wall_Dark" :!type "Material Object Reference"))
    (`PrimitiveComponent.SetMaterial` _returnvalue 0 _returnvalue_2)
    (`KismetArrayLibrary.Array_Add` (`self.Field_material`) _returnvalue_2)))