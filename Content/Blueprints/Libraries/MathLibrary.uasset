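; Math function library for a board with nine-wide indexing and 400-unit cells, plus a random colour helper.
; Converts between flat index, world position and RC (a two-digit, one-based row/column code), with "200" variants offset to cell centres.
; Quarter-turn rotation helpers invert a 0–3 value, wrap it by one turn, or look it up by RC in parallel emitting-board-state arrays.
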(fn `Index -> Position`
  (params (Int :type Integer))
  (returns (ReturnValue :type "Vector Structure"))
  (return (`KismetMathLibrary.MakeVector` (* (/ Int 9) 400.0) (* (mod Int 9) 400.0) 0.0)))

(fn `Index -> Position 200`
  (params (Int :type Integer))
  (returns (ReturnValue :type "Vector Structure"))
  (return (+ (`self.Index -> Position` Int) (200.0 200.0 0.0))))

(fn `Index -> RC`
  (params (A :type Integer))
  (returns (ReturnValue :type Integer))
  (return (+ (* (+ (/ A 9) 1) 10) (+ (mod A 9) 1))))

(fn `NormRotCalc`
  (params (CalcedRot :type Integer))
  (returns (NormedRot :type Integer))
  (bind _returnvalue (select `bool` (< CalcedRot 0) :`false` CalcedRot :`true` (+ CalcedRot 4)))
  (return (select `bool` (> _returnvalue 3) :`false` _returnvalue :`true` (- _returnvalue 4))))

(fn `Position -> Index`
  (params (A :type "Vector Structure"))
  (returns (ReturnValue :type Integer))
  (return (+ (* (`KismetMathLibrary.FFloor` (.x (/ A (400.0 400.0 1.0)))) 9) (`KismetMathLibrary.FFloor` (.y (/ A (400.0 400.0 1.0)))))))

(fn `Position -> RC`
  (params (A :type "Vector Structure"))
  (returns (ReturnValue :type Integer))
  (return (+ (* (+ (`KismetMathLibrary.FFloor` (.x (/ A (400.0 400.0 1.0)))) 1) 10) (+ (`KismetMathLibrary.FFloor` (.y (/ A (400.0 400.0 1.0)))) 1))))

(fn `RandomColor`
  (returns (ColorOut :type "LinearColor Structure"))
  (return (make `LinearColor` (`KismetMathLibrary.RandomFloatInRange` 0.0 1.0) (`KismetMathLibrary.RandomFloatInRange` 0.0 1.0) (`KismetMathLibrary.RandomFloatInRange` 0.0 1.0) 1.0)))

(fn `RC -> Position`
  (params (A :type Integer))
  (returns (Vector :type "Vector Structure"))
  (bind _returnvalue (/ A 10))
  (return (`KismetMathLibrary.MakeVector` (* (mod (- _returnvalue 1) 10) 400.0) (* (mod (- (- A (* _returnvalue 10)) 1) 10) 400.0))))

(fn `RC -> Position 200`
  (params (A :type Integer))
  (returns (ReturnValue :type "Vector Structure"))
  (return (+ (`self.RC -> Position` A) (200.0 200.0 0.0))))

(fn `RC -> Rot`
  (params (EmittingBoardStateRC :type "Array of Integer") (RC :type Integer) (EmittingBoardStateRot :type "Array of Integer"))
  (returns (Rot :type Integer))
  (locals (EmittingBoardStateRCLOCACL :type "Array of Integer") (EmittingBoardStateRotLOCAL :type "Array of Integer") (RCLOCAL :type Integer))
  (set `local.EmittingBoardStateRCLOCACL` EmittingBoardStateRC)
  (set `local.RCLOCAL` RC)
  (set `local.EmittingBoardStateRotLOCAL` EmittingBoardStateRot)
  (return (`|GetArrayItem` (`local.EmittingBoardStateRotLOCAL`) (`KismetArrayLibrary.Array_Find` (`local.EmittingBoardStateRCLOCACL`) (`local.RCLOCAL`)))))

(fn `RC -> Rot -> Inv`
  (params (EmittingBoardStateRC :type "Array of Integer") (RC :type Integer) (EmittingBoardStateRot :type "Array of Integer"))
  (returns (Rot :type Integer))
  (return (`self.Rot -> Inv` (`self.RC -> Rot` EmittingBoardStateRC RC EmittingBoardStateRot))))

(fn `Rot -> Inv`
  (params (Rot :type Integer))
  (returns (Inv :type Integer))
  (return (select `bool` (> Rot 1) :`false` (+ Rot 2) :`true` (- Rot 2))))